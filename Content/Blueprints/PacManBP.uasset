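; Player-controlled Pac-Man actor that eats tablets for points, loses lives to ghosts and respawns at its origin.
; Axis input sets a direction when a line trace finds no "wall"-named actor, and Tick moves and animates it until blocked.
; A self-re-entering Gate steps through timed GameModes, interrupted by super tablets that temporarily let it kill IGhost actors.
; The last death triggers no game-over handling, and the wind logic is unwired.
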(event EventBeginPlay
  (bind _returnvalue (UserInterface|CreateWidget "/Game/HUD/ScoreWidgetBP.ScoreWidgetBP_C" (Game|GetPlayerController 0)))
  (UserInterface|Viewport|AddtoViewport _returnvalue 0)
  (CallFunction|Start))

(event EventTick
  (params (DeltaSeconds :type Float%20%28single-precision%29))
  (bind _skeletalmesh (Variables|Default|GetSkeletalMesh))
  (bind _return (CallFunction|ExistWall (Variables|Default|GetDirection))) ; Check if there wall
  (if _return
    ;[1 1 1] Stop Animation
    (Audio|Components|Audio|Stop _skeletalmesh)
    (elif (Variables|Default|GetReady)
      ;[1 1 1] Movement
      (bind _location (CallFunction|GetNewLocation))
      (Transformation|SetActorLocation _location false false)
      ;[1 1 1] Play Animation
      (Audio|Components|Audio|Play _skeletalmesh true)
      (Components|Timeline|SetPlayRate _skeletalmesh 5.0))))

(event Input|AxisEvents|InputAxisMoveForward
  (params (AxisValue :type Float%20%28single-precision%29))
  ;[1 1 1] Controls
  (CallFunction|SetNewLocationRotation "1.000000, 0, 0" AxisValue))

(event Input|AxisEvents|InputAxisMoveRight
  (params (AxisValue :type Float%20%28single-precision%29))
  ;[1 1 1] Controls
  (CallFunction|SetNewLocationRotation "0,1.000000, 0" AxisValue))

(event Custom|Start
  ;[1 1 1] Event Start
  (bind _output_get (Variables|Default|SetPlaceOrigin (Transformation|GetActorLocation)))
  (Audio|PlaySoundatLocation "/Game/Sounds/pacman_beginning_S.pacman_beginning_S" _output_get)
  ;;[1 1 1] Ready delay
  (Utilities|FlowControl|Delay 3.0)
  (Variables|Default|SetReady true)
  (CallFunction|Gate))

(event Custom|Revive
  (bind _skeletalmesh (Variables|Default|GetSkeletalMesh))
  ;[1 1 1] Revive
  (Utilities|FlowControl|Delay 1.6)
  (Class|SkinnedMeshComponent|SetSkeletalMesh _skeletalmesh "/Game/Meshs/Teste_7.Teste_7" false)
  (Components|Animation|SetAnimation _skeletalmesh "/Game/Meshs/Teste_7_Anim.Teste_7_Anim")
  (bind _output_get (Variables|Default|SetDirection "0.000000,-1.000000, 0"))
  (Transformation|SetActorLocation (Variables|Default|GetPlaceOrigin) false false)
  (Transformation|SetRelativeRotation _skeletalmesh (Math|Conversions|RotationFromXVector _output_get) false false)
  (Variables|Default|SetGameMode 0)
  (CallFunction|Start))

(event Custom|Close%20Gate
  ;[1 1 1] Gate
  (Utilities|FlowControl|Gate false) ; enters at Close
)

(event Custom|Gate
  ;[1 1 1] Gate
  (Utilities|FlowControl|Sequence
    (:then_0
      (goto _label Open))
    (:then_1
      (Utilities|FlowControl|Gate false :!label _label
        (:Exit
          (if (< (Variables|Default|GetGMCount) 8)
            (Variables|Default|SetGameMode (Utilities|Array|Get(acopy) (Variables|Default|GetGameModes) (Variables|Default|GetGMCount)))
            (Utilities|FlowControl|Delay (Utilities|Array|Get(acopy) (Variables|Default|GetGameTime) (Variables|Default|GetGMCount)))
            (bind _result (Math|Integer|IncrementInt (Variables|Default|GetGMCount))
              (:%20%20
                (Variables|Default|SetGMCount _result)
                (if (and (Variables|Default|GetReady) (!= (Variables|Default|GetGameMode) 2))
                  (goto _label)
                  (else
                    (CallFunction|CloseGate)))))
            (else
              (CallFunction|CloseGate))))))))

(event OnComponentBeginOverlap(Collider)
  (params (OverlappedComponent :type Primitive%20Component%20Object%20Reference) (OtherActor :type Actor%20Object%20Reference) (OtherComp :type Primitive%20Component%20Object%20Reference) (OtherBodyIndex :type Integer) (bFromSweep :type Boolean) (SweepResult :type Hit%20Result%20Structure%20%28by%20ref%29))
  ;[1 1 1] Death
  (bind _asighost (Utilities|Casting|CastToIGhost OtherActor)
    (:then
      (if (!= (Variables|Default|GetGameMode) 2)
        (CallFunction|Death)
        (else
          (Default|Die _asighost))))
    (:CastFailed
      (Utilities|Casting|CastToTablet_DM_BP OtherActor
        (:then
          (Audio|PlaySound2D "/Game/Sounds/pacman_chomp_S.pacman_chomp_S")
          (Variables|Default|SetGamePoints (+ (Variables|Default|GetGamePoints) 10)))
        (:CastFailed
          ;[1 1 1] Super power
          (Utilities|Casting|CastToSuper_Tablet_DM_BP OtherActor)
          (Audio|PlaySound2D "/Game/Sounds/pacman_chomp_S.pacman_chomp_S")
          (CallFunction|CloseGate)
          (Variables|Default|SetGameMode 2)
          (Utilities|FlowControl|Delay 7.0)
          (CallFunction|Gate))))))

(event Custom|Wind%20Control)

(fn ConstructionScript)

(fn SetNewLocationRotation
  (params (Axis :type Vector) (Direction :type Float%20%28single-precision%29))
  (bind _returnvalue (* Axis Direction))
  (if (!= Direction 0.0)
    (bind _return (CallFunction|ExistWall _returnvalue))
    (if (not _return)
      (Transformation|SetRelativeRotation (Variables|Default|GetSkeletalMesh) (Math|Conversions|RotationFromXVector _returnvalue) false false)
      (Variables|Default|SetDirection _returnvalue)
      (return))))

(fn ExistWall
  (params (Direction :type Vector))
  (bind _returnvalue (Transformation|GetActorLocation))
  (bind _outhit (Collision|LineTraceByChannel _returnvalue (+ (* Direction 6e+01) _returnvalue) "TraceTypeQuery1" false 0 "None"))
  (return (Utilities|String|Contains (Utilities|GetDisplayName (.HitActor (Collision|BreakHitResult _outhit))) "wall")))

(fn GetNewLocation
  (return (+ (* (Variables|Default|GetDirection) (Variables|Default|GetVelocity)) (Transformation|GetActorLocation))))

(fn Death
  (bind _skeletalmesh (Variables|Default|GetSkeletalMesh))
  (bind _result (Math|Integer|DecrementInt (Variables|Default|GetLifes))
    (:%20%20
      (bind _output_get (Variables|Default|SetLifes _result))
      (if (not (== _output_get 0))
        (Class|SkinnedMeshComponent|SetSkeletalMesh _skeletalmesh "/Game/Meshs/Teste_6_Morte_.Teste_6_Morte_" false)
        (Components|Animation|SetAnimation _skeletalmesh "/Game/Meshs/Teste_6_Morte__Anim.Teste_6_Morte__Anim")
        (Components|Timeline|SetPlayRate _skeletalmesh 1e+03)
        (Transformation|SetRelativeRotation _skeletalmesh "0.000000,0.000000,90.000000" false false)
        (Audio|PlaySound2D "/Game/Sounds/pacman_death.pacman_death")
        (Variables|Default|SetReady false)
        (Variables|Default|SetGameMode 3)
        (Variables|Default|SetGMCount 0)
        (CallFunction|CloseGate)
        (CallFunction|Revive)))))
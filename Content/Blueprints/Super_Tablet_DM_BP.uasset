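; Super tablet pickup for a Pac-Man style game that shatters and awards bonus points when the player overlaps it.
; On actor overlap with PacManBP, it applies heavy radius damage with a strong impulse to its Destructible component and adds to the player's GamePoints.
; An IsDetroyed flag blocks repeat scoring, and the trailing Delay leads to no further action, so the actor is never removed here.
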(event Collision|EventActorBeginOverlap
  (params (OtherActor :type Actor%20Object%20Reference))
  (if (not (Variables|Default|GetisDetroyed))
    (bind _aspac_man_bp (Utilities|Casting|CastToPacManBP OtherActor))
    (Class|DestructibleComponent|ApplyRadiusDamage (Variables|Default|GetDestructible) 1e+04 (Transformation|GetActorLocation) 5e+03 1e+04 true)
    (Variables|/Game/Blueprints/PacManBP.PacManBP_C|SetGamePoints _aspac_man_bp (+ (Variables|/Game/Blueprints/PacManBP.PacManBP_C|GetGamePoints _aspac_man_bp) 50))
    (Variables|Default|SetisDetroyed true)
    (Utilities|FlowControl|Delay 1.0)))

(fn ConstructionScript)
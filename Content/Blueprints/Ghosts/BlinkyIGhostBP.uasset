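; Blinky, a Pac-Man ghost Blueprint that specialises a parent ghost class by directly targeting the player.
; Chase returns Pac-Man's current location as the target.
; BeginPlay registers Blinky on PacManBP, fills a hardcoded DLocations waypoint list and holds Wait for a short startup delay.
; Tick runs parent logic only while Move is false; Divide is empty and ResetDivide just resets Count.
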(event EventBeginPlay
  (|CallParentFunction)
  (bind _aspac_man_bp (Utilities|Casting|CastToPacManBP (Game|Player|GetPlayerPawn 0))
    (:then
      (Variables|/Game/Blueprints/PacManBP.PacManBP_C|SetBlinkyRef _aspac_man_bp self))
    (:CastFailed
      _))
  (Variables|Default|SetDLocations (Utilities|Array|MakeArray "-23622.000000,-24418.000000,76.000000" "-23622.000000,-23780.000000,76.000000" "-23409.000000,-23780.000000,76.000000" "-23409.000000,-23501.000000,76.000000" "-23630.000000,-23501.000000,76.000000" "-24428.000000,-23781.000000,76.000000"))
  (Variables|Default|SetWait true)
  (Utilities|FlowControl|Delay 3.0)
  (Variables|Default|SetWait false))

(event Collision|EventActorBeginOverlap
  (params (OtherActor :type Actor%20Object%20Reference)))

(event EventTick
  (params (DeltaSeconds :type Float%20%28single-precision%29))
  (if (not (Variables|Default|GetMove))
    (|CallParentFunction DeltaSeconds)))

(fn ConstructionScript
  (|CallParentFunction))

(fn Chase
  (bind _aspac_man_bp (Utilities|Casting|CastToPacManBP (Game|Player|GetPlayerPawn 0)))
  (return (Transformation|GetActorLocation _aspac_man_bp)))

(fn Divide
  (return))

(fn ResetDivide
  (Variables|Default|SetCount 1)
  (return true))
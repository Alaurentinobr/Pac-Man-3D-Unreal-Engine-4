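; Pinky ghost for a Pac-Man game, a child Blueprint that specialises a parent ghost's behaviour.
; BeginPlay fills a fixed list of DLocations waypoints and holds back the parent Tick for a few seconds.
; Chase targets a point just ahead of Pac-Man along its direction, shifting it sideways by the mesh's right vector when a wall blocks that direction.
; Divide is an empty function.
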(event Collision|EventActorBeginOverlap
  (params (OtherActor :type Actor%20Object%20Reference)))

(event EventBeginPlay
  (|CallParentFunction)
  (Variables|Default|SetDLocations (Utilities|Array|MakeArray "-23625.000000,-24581.000000,76.000000" "-23412.000000,-24581.000000,76.000000" "-23412.000000,-24860.000000,76.000000" "-23628.000000,-24860.000000,76.000000" "-23628.000000,-24583.000000,76.000000" "-24431.000000,-24583.000000,76.000000"))
  (Variables|Default|SetWait true)
  (Utilities|FlowControl|Delay 7.0)
  (Variables|Default|SetWait false))

(event EventTick
  (params (DeltaSeconds :type Float%20%28single-precision%29))
  (if (not (Variables|Default|GetWait))
    (|CallParentFunction 0.0)))

(fn ConstructionScript
  (|CallParentFunction))

(fn Chase
  (bind _aspac_man_bp (Utilities|Casting|CastToPacManBP (Game|Player|GetPlayerPawn 0)))
  (bind _return (Default|ExistWall _aspac_man_bp (Variables|/Game/Blueprints/PacManBP.PacManBP_C|GetDirection _aspac_man_bp)))
  (if _return
    (return (+ (* (Math|Vector|GetRightVector (Variables|/Script/Engine.SceneComponent|GetRelativeRotation (Variables|/Game/Blueprints/PacManBP.PacManBP_C|GetSkeletalMesh _aspac_man_bp))) -1e+02) (+ (Transformation|GetActorLocation _aspac_man_bp) (* (Variables|/Game/Blueprints/PacManBP.PacManBP_C|GetDirection _aspac_man_bp) 1e+02))))
    (else
      (return (+ (Transformation|GetActorLocation _aspac_man_bp) (* (Variables|/Game/Blueprints/PacManBP.PacManBP_C|GetDirection _aspac_man_bp) 1e+02))))))

(fn Divide
  (return))
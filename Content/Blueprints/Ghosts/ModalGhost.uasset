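; Base ghost Blueprint for a Pac-Man game, with placeholder Chase, Scared and Tick2 hooks that appear meant for child ghosts to override.
; Tick reads the player PacManBP's GameMode, shows the mesh outside mode 3 and switches on the mode when Move and IsDeath are false, then calls Tick2.
; A gate on OnChase drives AIMoveTo toward the Chase result, a zero vector here, and CloseOnChase closes it.
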(event Custom|Tick%202
  (params (Delta%20Segunds :type Float%20%28single-precision%29)))

(event Custom|OnChase
  (Utilities|FlowControl|Sequence
    (:then_0
      (goto _label Open))
    (:then_1
      (Utilities|FlowControl|Gate true :!label _label
        (:Exit
          (bind _chase_location (CallFunction|Chase))
          (AI|AIMoveTo 0 _chase_location 0 5.0 false))))))

(event Custom|Close%20OnChase
  (Utilities|FlowControl|Gate true) ; enters at Close
)

(event EventTick
  (params (DeltaSeconds :type Float%20%28single-precision%29))
  (Utilities|FlowControl|Sequence
    (:then_0
      (bind _aspac_man_bp (Utilities|Casting|CastToPacManBP (Game|Player|GetPlayerPawn 0)))
      (if (!= (Variables|/Game/Blueprints/PacManBP.PacManBP_C|GetGameMode _aspac_man_bp) 3)
        (Rendering|SetVisibility (Variables|Default|GetStaticMesh) true true)
        (if (and (not (Variables|Default|GetMove)) (not (Variables|Default|GetisDeath)))
          (switch int (Variables|/Game/Blueprints/PacManBP.PacManBP_C|GetGameMode _aspac_man_bp)))))
    (:then_1
      (CallFunction|Tick2 0.0))))

(fn ConstructionScript)

(fn Chase
  (return "0, 0, 0"))

(fn Scared)
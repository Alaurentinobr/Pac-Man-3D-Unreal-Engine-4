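; Clyde ghost for a Pac-Man game, a child Blueprint that overrides the parent's Chase targeting.
; Chase returns the player's location, or a hard-coded retreat waypoint selected by an index while RunAway is set.
; Sphere hits set RunAway on contact with Pac-Man and clear it on any other actor.
; Scared defers to the parent, and the waypoint index is never advanced here.
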(event OnComponentHit(Sphere)
  (params (HitComponent :type Primitive%20Component%20Object%20Reference) (OtherActor :type Actor%20Object%20Reference) (OtherComp :type Primitive%20Component%20Object%20Reference) (NormalImpulse :type Vector :default "0, 0, 0") (Hit :type Hit%20Result%20Structure%20%28by%20ref%29))
  (Utilities|Casting|CastToPacManBP OtherActor
    (:then
      (Variables|Default|SetRunAway true))
    (:CastFailed
      (Variables|Default|SetRunAway false))))

(event EventBeginPlay
  (|CallParentFunction)
  (|CallParentFunction)
  (Variables|Default|SetDLocations (Utilities|Array|MakeArray "-24592.000000,-24567.000000,76.000000" "-24740.000000,-24567.000000,76.000000" "-24740.000000,-24826.000000,76.000000" "-24910.000000,-24826.000000,76.000000" "-24910.000000,-24275.000000,76.000000" "-24749.000000,-24416.000000,76.000000"))
  (Variables|Default|SetWait true)
  (Utilities|FlowControl|Delay 0.0)
  (Variables|Default|SetWait false))

(event Collision|EventActorBeginOverlap
  (params (OtherActor :type Actor%20Object%20Reference)))

(event EventDivideEnter)

(event EventTick
  (params (DeltaSeconds :type Float%20%28single-precision%29))
  (|CallParentFunction 0.0))

(fn ConstructionScript
  (|CallParentFunction))

(fn Chase
  (bind _i (Variables|Default|Geti))
  (bind _aspac_man_bp (Utilities|Casting|CastToPacManBP (Game|Player|GetPlayerPawn 0)))
  (if (Variables|Default|GetRunAway)
    (if (< _i 6)
      (return (Utilities|Array|Get(acopy) (Variables|Default|GetDLocations) _i)))
    (else
      (return (Transformation|GetActorLocation _aspac_man_bp)))))

(fn Scared
  (bind _location (|CallParentFunction))
  (return _location))
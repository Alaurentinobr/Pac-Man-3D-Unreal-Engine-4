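; Red ghost (Blinky-style) Blueprint for a Pac-Man game, a child class that supplies this ghost's chase targeting.
; Its Chase function casts the player pawn to PacManBP and returns that actor's current location as a direct pursuit target.
; BeginPlay, Tick and construction defer to the parent class; BeginPlay also casts the player pawn but does nothing with the result.
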(event EventBeginPlay
  (|CallParentFunction)
  (Utilities|Casting|CastToPacManBP (Game|Player|GetPlayerPawn 0)))

(event Collision|EventActorBeginOverlap
  (params (OtherActor :type Actor%20Object%20Reference)))

(event EventTick
  (params (DeltaSeconds :type Float%20%28single-precision%29))
  (|CallParentFunction DeltaSeconds))

(fn ConstructionScript
  (|CallParentFunction))

(fn Chase
  (bind _aspac_man_bp (Utilities|Casting|CastToPacManBP (Game|Player|GetPlayerPawn 0)))
  (return (Transformation|GetActorLocation _aspac_man_bp)))
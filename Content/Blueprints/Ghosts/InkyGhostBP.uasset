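; Inky ghost Blueprint for a Pac-Man game, built on a parent ghost class and held idle for a few seconds after BeginPlay before the parent Tick runs.
; It fills a fixed list of DLocations waypoints and overrides Chase to target its own position mirrored through a point ahead of Pac-Man.
; When Pac-Man faces a wall, the target shifts along his mesh's right vector.
; Divide is empty.
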(event EventBeginPlay
  (|CallParentFunction)
  (Variables|Default|SetDLocations (Utilities|Array|MakeArray "-24742.000000,-23777.000000,76.000000" "-24742.000000,-23510.000000,76.000000" "-24910.000000,-23510.000000,76.000000" "-24910.000000,-24096.000000,76.000000" "-24753.000000,-24096.000000,76.000000" "-24602.000000,-23945.000000,76.000000"))
  (Variables|Default|SetWait true)
  (Utilities|FlowControl|Delay 7.0)
  (Variables|Default|SetWait false))

(event Collision|EventActorBeginOverlap
  (params (OtherActor :type Actor%20Object%20Reference)))

(event EventTick
  (params (DeltaSeconds :type Float%20%28single-precision%29))
  (if (not (Variables|Default|GetWait))
    (|CallParentFunction DeltaSeconds)))

(fn ConstructionScript
  (|CallParentFunction))

(fn Chase
  (bind _aspac_man_bp (Utilities|Casting|CastToPacManBP (Game|Player|GetPlayerPawn 0)))
  (bind _return (Default|ExistWall _aspac_man_bp (Variables|/Game/Blueprints/PacManBP.PacManBP_C|GetDirection _aspac_man_bp)))
  (if _return
    (return (+ (* (Math|Vector|GetRightVector (Variables|/Game/Blueprints/PacManBP.PacManBP_C|GetSkeletalMesh _aspac_man_bp)) 100) (- (* (+ (Transformation|GetActorLocation _aspac_man_bp) (* (Variables|/Game/Blueprints/PacManBP.PacManBP_C|GetDirection _aspac_man_bp) 80)) 2) (Transformation|GetActorLocation))))
    (else
      (return (- (* (+ (Transformation|GetActorLocation _aspac_man_bp) (* (Variables|/Game/Blueprints/PacManBP.PacManBP_C|GetDirection _aspac_man_bp) 80)) 2) (Transformation|GetActorLocation))))))

(fn Divide
  (return))
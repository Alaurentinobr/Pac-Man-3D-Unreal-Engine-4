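; Base Pac-Man ghost that switches between scatter (Divide), chase and scared movement based on the player PacManBP's GameMode, polled on Tick.
; Gated AIMoveTo branches walk DLocations waypoints, seek the Chase function's point (a zero-vector stub here) or pick random navigable points.
; Die, also bound to Z, clears the mesh and paths to the world origin to revive.
; GameMode 3 hides the ghost, closes the gates and teleports it to its start.
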(event Custom|Restart
  (Rendering|SetVisibility (Variables|Default|GetSkeletalMesh) false true)
  (CallFunction|CloseDelegates)
  (Transformation|SetActorLocation (Variables|Default|GetPlaceOrigin) false false)
  (Variables|Default|SetMove false)
  (Variables|Default|SetisDeath false))

(event Custom|Close%20Delegates
  (CallFunction|DivideClose)
  (CallFunction|ChaseClose)
  (CallFunction|ScaredClose))

(event Custom|Die
  (Variables|Default|SetisDeath true)
  (Class|SkinnedMeshComponent|SetSkeletalMesh (Variables|Default|GetSkeletalMesh) 0 true)
  (AI|AIMoveTo 0 (Variables|Default|GetReviveLocation) 0 5e+01 false
    (:then
      (Variables|Default|SetMove true))
    (:OnSuccess
      (Class|SkinnedMeshComponent|SetSkeletalMesh (Variables|Default|GetSkeletalMesh) "/Game/Meshs/Teste_7.Teste_7" true)
      (Variables|Default|SetisDeath false)
      (Variables|Default|SetMove false))))

(event Custom|Scared%20Enter
  (Utilities|FlowControl|Sequence
    (:then_0
      (goto _label Open))
    (:then_1
      (Utilities|FlowControl|Gate true :!label _label
        (:Exit
          (bind _location (CallFunction|Scared))
          (AI|AIMoveTo self _location 0 3e+01 false
            (:then
              (Variables|Default|SetMove true))
            (:OnSuccess
              (Variables|Default|SetMove false :!label _label_2))
            (:OnFail
              (goto _label_2))))))))

(event Custom|Scared%20Close
  (Utilities|FlowControl|Gate true) ; enters at Close
)

(event Custom|Divide%20Enter
  (bind _dlocations (Variables|Default|GetDLocations))
  (bind _returnvalue (Utilities|Array|Length _dlocations))
  (Utilities|FlowControl|Sequence
    (:then_0
      (goto _label Open))
    (:then_1
      (Utilities|FlowControl|Gate true :!label _label
        (:Exit
          (bind _aspac_man_bp (Utilities|Casting|CastToPacManBP (Game|Player|GetPlayerPawn 0)))
          (if (and (== (Variables|/Game/Blueprints/PacManBP.PacManBP_C|GetGameMode _aspac_man_bp) 0) (and (!= _returnvalue 0) (< (Variables|Default|GetCount) _returnvalue)))
            (AI|AIMoveTo self (Utilities|Array|Get(acopy) (Variables|Default|GetDLocations) (Variables|Default|GetCount)) 0 3e+01 false
              (:then
                (Variables|Default|SetMove true))
              (:OnSuccess
                (bind _result (Math|Integer|IncrementInt (Variables|Default|GetCount))
                  (:%20%20
                    (Variables|Default|SetCount _result)
                    (Variables|Default|SetMove true)
                    (goto _label))))
              (:OnFail
                (Variables|Default|SetMove false :!label _label_2)
                (Padrão|ResetDivide)))
            (else
              (goto _label_2))))))))

(event Custom|Divide%20Close
  (bind _dlocations (Variables|Default|GetDLocations))
  (bind _returnvalue (Utilities|Array|Length _dlocations))
  (Utilities|FlowControl|Gate true) ; enters at Close
)

(event Custom|Chase%20Enter
  (Utilities|FlowControl|Sequence
    (:then_0
      (goto _label Open))
    (:then_1
      (Utilities|FlowControl|Gate true :!label _label
        (:Exit
          (bind _location (CallFunction|Chase))
          (AI|AIMoveTo self _location 0 3e+01 false))))))

(event Custom|Chase%20Close
  (Utilities|FlowControl|Gate true) ; enters at Close
)

(event EventBeginPlay
  (Variables|Default|SetPlaceOrigin (Transformation|GetActorLocation))
  (Variables|Default|SetReviveLocation "0, 0, 0"))

(event EventTick
  (params (DeltaSeconds :type Float%20%28single-precision%29))
  (bind _aspac_man_bp (Utilities|Casting|CastToPacManBP (Game|Player|GetPlayerPawn 0)))
  (if (!= (Variables|/Game/Blueprints/PacManBP.PacManBP_C|GetGameMode _aspac_man_bp) 3)
    (Rendering|SetVisibility (Variables|Default|GetSkeletalMesh) true true)
    (if (and (and (Variables|/Game/Blueprints/PacManBP.PacManBP_C|GetReady _aspac_man_bp) (not (Variables|Default|GetisDeath))) (not (Variables|Default|GetMove)))
      (Padrão|ResetDivide)
      (switch int (Variables|/Game/Blueprints/PacManBP.PacManBP_C|GetGameMode _aspac_man_bp)
        (:Default
          (CallFunction|ScaredEnter))
        (:0
          (CallFunction|DivideEnter))
        (:1
          (CallFunction|ChaseEnter))))
    (else
      (CallFunction|Restart))))

(event Input|KeyboardEvents|Z
  (params (Key :type Key%20Structure :default "AnyKey"))
  (:Pressed
    (CallFunction|Die)))

(fn ConstructionScript)

(fn Chase
  (return "0, 0, 0"))

(fn Scared
  (return (Class|NavigationSystem|GetRandomPointinNavigableRadius (Transformation|GetActorLocation) 1e+03)))

(fn ResetDivide
  (Variables|Default|SetCount 0)
  (return true))
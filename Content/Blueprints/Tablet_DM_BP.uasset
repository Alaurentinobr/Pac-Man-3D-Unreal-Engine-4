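; Tablet_DM_BP is a destructible pellet that Pac-Man collects for points.
; When a PacManBP overlaps it, heavy full radius damage shatters its Destructible component and 10 is added to that player's GamePoints.
; An IsDestroyed flag prevents repeat scoring, and after a short delay the Destructible component is hidden rather than the actor being destroyed.
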(event Collision|EventActorBeginOverlap
  (params (OtherActor :type Actor%20Object%20Reference))
  (if (not (Variables|Default|GetisDestroyed))
    (bind _aspac_man_bp (Utilities|Casting|CastToPacManBP OtherActor))
    (Class|DestructibleComponent|ApplyRadiusDamage (Variables|Default|GetDestructible) 1e+04 (Transformation|GetActorLocation) 5e+03 1e+04 true)
    (Variables|/Game/Blueprints/PacManBP.PacManBP_C|SetGamePoints _aspac_man_bp (+ (Variables|/Game/Blueprints/PacManBP.PacManBP_C|GetGamePoints _aspac_man_bp) 10))
    (Variables|Default|SetisDestroyed true)
    (Utilities|FlowControl|Delay 5.0)
    (Rendering|SetVisibility (Variables|Default|GetDestructible) false false)))

(event Collision|EventHit
  (params (MyComp :type Primitive%20Component%20Object%20Reference) (Other :type Actor%20Object%20Reference) (OtherComp :type Primitive%20Component%20Object%20Reference) (bSelfMoved :type Boolean) (HitLocation :type Vector :default "0, 0, 0") (HitNormal :type Vector :default "0, 0, 0") (NormalImpulse :type Vector :default "0, 0, 0") (Hit :type Hit%20Result%20Structure%20%28by%20ref%29)))

(fn ConstructionScript)